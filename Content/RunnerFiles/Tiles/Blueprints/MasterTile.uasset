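; MasterTile is a runner tile actor, apparently the base for tiles, that keeps the track going as the player moves.
; When the ThirdPersonCharacter overlaps its Box, it asks ThirdPersonGameMode to spawn another tile.
; It then adds points scaled by the game mode's points multiplier, prints the total, and destroys itself after a short delay.
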(event `self.Box.OnComponentBeginOverlap`
  (params (OverlappedComponent :type "PrimitiveComponent Object Reference") (OtherActor :type "Actor Object Reference") (OtherComp :type "PrimitiveComponent Object Reference") (OtherBodyIndex :type Integer) (bFromSweep :type Boolean) (SweepResult :type "HitResult Structure (by ref)"))
  (cast `/Game/ThirdPersonBP/Blueprints/ThirdPersonCharacter` OtherActor)
  ;[1 1 1] Spawn plataformas
  (bind _asthird_person_game_mode (cast `/Game/ThirdPersonBP/Blueprints/ThirdPersonGameMode` (`GameplayStatics.GetGameMode`)))
  (`/Game/ThirdPersonBP/Blueprints/ThirdPersonGameMode.SpawnTile` _asthird_person_game_mode)
  (bind _output_get (set `/Game/ThirdPersonBP/Blueprints/ThirdPersonGameMode.CurrentPoints` (+ (* 15 (`/Game/ThirdPersonBP/Blueprints/ThirdPersonGameMode.PointsMultiplayer` _asthird_person_game_mode)) (`/Game/ThirdPersonBP/Blueprints/ThirdPersonGameMode.CurrentPoints` _asthird_person_game_mode)) _asthird_person_game_mode))
  (`KismetSystemLibrary.PrintString` (`KismetStringLibrary.Conv_IntToString` _output_get))
  ;[1 1 1] Destruye las plataformas
  (`KismetSystemLibrary.Delay` 0.5)
  (`self.K2_DestroyActor`))

(fn `UserConstructionScript`)