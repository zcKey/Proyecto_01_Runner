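; Floor tile for a three-lane runner that populates itself with random obstacles and pickups on BeginPlay.
; SpawnObstacles rolls per lane in sequence for walls, spikes, barriers, coins, magnets or coin boxes; an empty roll also skips remaining lanes.
; When the character overlaps its Box, the GameMode spawns another tile and adds multiplied points.
; The overlap also raises player walk speed within a clamped range, then destroys the tile after a short delay.
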(event `self.ReceiveBeginPlay`
  (`self.SpawnObstacles`))

(event `self.Box.OnComponentBeginOverlap`
  (params (OverlappedComponent :type "PrimitiveComponent Object Reference") (OtherActor :type "Actor Object Reference") (OtherComp :type "PrimitiveComponent Object Reference") (OtherBodyIndex :type Integer) (bFromSweep :type Boolean) (SweepResult :type "HitResult Structure (by ref)"))
  (cast `/Game/ThirdPersonBP/Blueprints/ThirdPersonCharacter` OtherActor)
  ;[1 1 1] Spawn plataformas
  (bind _asthird_person_game_mode (cast `/Game/ThirdPersonBP/Blueprints/ThirdPersonGameMode` (`GameplayStatics.GetGameMode`)))
  (`/Game/ThirdPersonBP/Blueprints/ThirdPersonGameMode.SpawnTile` _asthird_person_game_mode)
  (bind _output_get (set `/Game/ThirdPersonBP/Blueprints/ThirdPersonGameMode.CurrentPoints` (+ (* 15 (`/Game/ThirdPersonBP/Blueprints/ThirdPersonGameMode.PointsMultiplayer` _asthird_person_game_mode)) (`/Game/ThirdPersonBP/Blueprints/ThirdPersonGameMode.CurrentPoints` _asthird_person_game_mode)) _asthird_person_game_mode))
  (`KismetSystemLibrary.PrintString` (`KismetStringLibrary.Conv_IntToString` _output_get))
  ;[1 1 1] Incrementamos la velocidad del player cada vez que se crean plataformas
  (bind _asthird_person_character (cast `/Game/ThirdPersonBP/Blueprints/ThirdPersonCharacter` (`GameplayStatics.GetPlayerCharacter` 0)))
  (bind _charactermovement (`Character.CharacterMovement` _asthird_person_character))
  (set `CharacterMovementComponent.MaxWalkSpeed` (`KismetMathLibrary.FClamp` (* (`CharacterMovementComponent.MaxWalkSpeed` _charactermovement) 1.01) 600.0 1200.0) _charactermovement)
  ;[1 1 1] Destruye las plataformas
  (`KismetSystemLibrary.Delay` 0.5)
  (`self.K2_DestroyActor`))

(fn `SpawnObstacles`
  (bind _returnvalue (`SceneComponent.K2_GetComponentToWorld` (`self.Lane_2`)))
  (bind _returnvalue_2 (`SceneComponent.K2_GetComponentToWorld` (`self.Lane_0`)))
  (bind _returnvalue_3 (`SceneComponent.K2_GetComponentToWorld` (`self.Lane_1`)))
  ;[1 1 1] Obstaculos lane_0
  (switch `int` (`KismetMathLibrary.RandomIntegerInRange` 0 6)
    (:`1`
      (`|SpawnActorFromClass` "/Game/RunnerFiles/Blueprints/BP_Wall.BP_Wall_C" _returnvalue_2 "Undefined" "OverrideRootScale" null null))
    (:`2`
      (`|SpawnActorFromClass` "/Game/RunnerFiles/Blueprints/BP_Spyke.BP_Spyke_C" _returnvalue_2 "Undefined" "OverrideRootScale" null null))
    (:`3`
      (`|SpawnActorFromClass` "/Game/RunnerFiles/Blueprints/BP_Coin.BP_Coin_C" _returnvalue_2 "Undefined" "OverrideRootScale" null null))
    (:`4`
      (`|SpawnActorFromClass` "/Game/RunnerFiles/Blueprints/BP_Magnet.BP_Magnet_C" _returnvalue_2 "Undefined" "OverrideRootScale" null null))
    (:`5`
      (`|SpawnActorFromClass` "/Game/RunnerFiles/Blueprints/BP_Box_coins.BP_Box_coins_C" _returnvalue_2 "Undefined" "OverrideRootScale" null null))
    (:`6`
      (`|SpawnActorFromClass` "/Game/RunnerFiles/Blueprints/BP_Barrier.BP_Barrier_C" _returnvalue_2 "Undefined" "OverrideRootScale" null null)))
  ;[1 1 1] Obstaculos lane_1
  (switch `int` (`KismetMathLibrary.RandomIntegerInRange` 0 6)
    (:`1`
      (`|SpawnActorFromClass` "/Game/RunnerFiles/Blueprints/BP_Wall.BP_Wall_C" _returnvalue_3 "Undefined" "OverrideRootScale" null null))
    (:`2`
      (`|SpawnActorFromClass` "/Game/RunnerFiles/Blueprints/BP_Spyke.BP_Spyke_C" _returnvalue_3 "Undefined" "OverrideRootScale" null null))
    (:`3`
      (`|SpawnActorFromClass` "/Game/RunnerFiles/Blueprints/BP_Coin.BP_Coin_C" _returnvalue_3 "Undefined" "OverrideRootScale" null null))
    (:`4`
      (`|SpawnActorFromClass` "/Game/RunnerFiles/Blueprints/BP_Magnet.BP_Magnet_C" _returnvalue_3 "Undefined" "OverrideRootScale" null null))
    (:`5`
      (`|SpawnActorFromClass` "/Game/RunnerFiles/Blueprints/BP_Box_coins.BP_Box_coins_C" _returnvalue_3 "Undefined" "OverrideRootScale" null null))
    (:`6`
      (`|SpawnActorFromClass` "/Game/RunnerFiles/Blueprints/BP_Barrier.BP_Barrier_C" _returnvalue_3 "Undefined" "OverrideRootScale" null null)))
  ;[1 1 1] Obstaculos lane_2
  (switch `int` (`KismetMathLibrary.RandomIntegerInRange` 0 6)
    (:`1`
      (`|SpawnActorFromClass` "/Game/RunnerFiles/Blueprints/BP_Wall.BP_Wall_C" _returnvalue "Undefined" "OverrideRootScale" null null))
    (:`2`
      (`|SpawnActorFromClass` "/Game/RunnerFiles/Blueprints/BP_Spyke.BP_Spyke_C" _returnvalue "Undefined" "OverrideRootScale" null null))
    (:`3`
      (`|SpawnActorFromClass` "/Game/RunnerFiles/Blueprints/BP_Coin.BP_Coin_C" _returnvalue "Undefined" "OverrideRootScale" null null))
    (:`4`
      (`|SpawnActorFromClass` "/Game/RunnerFiles/Blueprints/BP_Magnet.BP_Magnet_C" _returnvalue "Undefined" "OverrideRootScale" null null))
    (:`5`
      (`|SpawnActorFromClass` "/Game/RunnerFiles/Blueprints/BP_Box_coins.BP_Box_coins_C" _returnvalue "Undefined" "OverrideRootScale" null null))
    (:`6`
      (`|SpawnActorFromClass` "/Game/RunnerFiles/Blueprints/BP_Barrier.BP_Barrier_C" _returnvalue "Undefined" "OverrideRootScale" null null))))

(fn `UserConstructionScript`)